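; Actor component that gives its owning Character a blink teleport along its last movement input.
; Trace steps back from maximum distance in capsule-sized increments, using sphere, line and capsule traces to find a clear path, ground and standing room.
; If no spot qualifies, the blink happens in place.
; BlinkStart hides the mesh, disables input and spawns Niagara effects, then a timer fires BlinkEnd to teleport and restore both.
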(event `self.ReceiveBeginPlay`
  (`|ExecutionSequence`
    (:`then_0`
      (bind _ascharacter (cast `Character` (`self.GetOwner`)))
      (bind _output_get (set `self.As Character` _ascharacter))
      (set `self.SK_Mesh` (`Character.Mesh` _output_get))
      (bind (_outradius _outhalfheight) (`CapsuleComponent.GetScaledCapsuleSize` (`Character.CapsuleComponent` _ascharacter)))
      (set `self.CapsuleRadius` _outradius)
      (set `self.CapsuleHalfHeight` _outhalfheight)
      (`self.UpdateBlink` (`self.BlinkDistance`)))))

(event `BlinkStart`
  ;[1 1 1] Blink
  (`SceneComponent.SetVisibility` (`self.SK_Mesh`) false true)
  (`Actor.DisableInput` (`self.As Character`) (`GameplayStatics.GetPlayerController` 0))
  (`NiagaraFunctionLibrary.SpawnSystemAtLocation` "/Game/Niagara/Blink/NS_Start.NS_Start" (`self.TeleportLocation`))
  (bind _returnvalue (`NiagaraFunctionLibrary.SpawnSystemAtLocation` "/Game/Niagara/Blink/NS_Middle.NS_Middle" (`self.TeleportLocation`)))
  (set `self.NS_MiddleRef` _returnvalue)
  (bind _returnvalue_2 (`KismetSystemLibrary.K2_SetTimerDelegate` (delegate `BlinkEnd`) (`self.BlinkDelay`)))
  (set `self.BlinkTimer` _returnvalue_2))

(event `BlinkEnd`
  ;[1 1 1] Blink
  (`SceneComponent.K2_SetWorldLocation` (`Character.CapsuleComponent` (`self.As Character`)) (`self.TeleportLocation`) false true)
  (`NiagaraFunctionLibrary.SpawnSystemAtLocation` "/Game/Niagara/Blink/NS_End.NS_End" (`SceneComponent.K2_GetComponentLocation` (`Character.CapsuleComponent` (`self.As Character`))))
  (`self.Deactivate` (`self.NS_MiddleRef`))
  (`SceneComponent.SetVisibility` (`self.SK_Mesh`) true true)
  (`Actor.EnableInput` (`self.As Character`) (`GameplayStatics.GetPlayerController` 0))
  (set `self.IsBlinking` false))

(event `Trace`
  (bind _as_character (`self.As Character`))
  (bind _returnvalue (`SceneComponent.K2_GetComponentLocation` (`Character.CapsuleComponent` _as_character)))
  (for _ (range (+ (`self.LastIndex`) 1)) :!label _label
    (bind (_outhit _returnvalue_2) (`KismetSystemLibrary.SphereTraceSingle` :`Start` (+ _returnvalue (0.0 0.0 100.0)) :`End` (+ (+ _returnvalue (* (`self.TempBlinkDistance`) (`KismetMathLibrary.Normal` (`PawnMovementComponent.GetLastInputVector` (`Character.CharacterMovement` _as_character))))) (0.0 0.0 100.0)) :`Radius` 20.0 :`TraceChannel` "TraceTypeQuery1" :`DrawDebugType` (`self.Draw Debug Type`)))
    (if _returnvalue_2
      (`self.UpdateTempBlinkDistance`)
      (else
        (bind (_bblockinghit _binitialoverlap _time _distance _location _impactpoint _normal _impactnormal _physmat _hitactor _hitcomponent _hitbonename _bonename _hititem _elementindex _faceindex _tracestart _traceend) (`GameplayStatics.BreakHitResult` _outhit))
        (bind (_outhit_2 _returnvalue_3) (`KismetSystemLibrary.LineTraceSingle` :`Start` (+ _traceend (0.0 0.0 100.0)) :`End` (+ _traceend (0.0 0.0 -300.0)) :`TraceChannel` "TraceTypeQuery1" :`DrawDebugType` (`self.Draw Debug Type`)))
        (if _returnvalue_3
          (bind (_bblockinghit_2 _binitialoverlap_2 _time_2 _distance_2 _location_2 _impactpoint_2 _normal_2) (`GameplayStatics.BreakHitResult` _outhit_2))
          (bind _returnvalue_4 (+ _location_2 (* _normal_2 100.0)))
          (bind (_outhit_3 _returnvalue_5) (`KismetSystemLibrary.CapsuleTraceSingle` :`Start` _returnvalue_4 :`End` _returnvalue_4 :`Radius` (* (`self.CapsuleRadius`) 1.2) :`HalfHeight` (* (`self.CapsuleHalfHeight`) 1.1) :`TraceChannel` "TraceTypeQuery1" :`DrawDebugType` (`self.Draw Debug Type`)))
          (if _returnvalue_5
            (`self.UpdateTempBlinkDistance`)
            (else
              (set `self.TeleportLocation` (`.TraceEnd` (`GameplayStatics.BreakHitResult` _outhit_3)))
              (`self.Break Blink Loop`)))
          (else
            (`self.UpdateTempBlinkDistance`))))))
  (set `self.TempBlinkDistance` (`self.BlinkDistance`))
  (if (not (`self.IsBlinking`))
    (set `self.TeleportLocation` (`SceneComponent.K2_GetComponentLocation` (`Character.CapsuleComponent` (`self.As Character`))))
    (set `self.IsBlinking` true)
    (`self.BlinkStart`)))

(event `Break Blink Loop`
  (if (not (`self.IsBlinking`))
    (set `self.IsBlinking` true)
    (`self.BlinkStart`)
    (goto _label :!via `Break`)))

(fn `DianeterOfCapsule`
  (returns (ReturnValue :type "Float (double-precision)"))
  (return (* (`self.CapsuleRadius`) 2.4)))

(fn `UpdateBlink`
  (params (TempBlinkDistance :type "Float (double-precision)"))
  (set `self.TempBlinkDistance` TempBlinkDistance)
  (set `self.LastIndex` (`KismetMathLibrary.FTrunc` (/ TempBlinkDistance (`self.DianeterOfCapsule`)))))