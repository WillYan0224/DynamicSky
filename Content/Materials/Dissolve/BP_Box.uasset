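; BP_Box is a volume actor that feeds an oriented box into materials, likely as the region for a dissolve effect.
; Its construction script writes the Cube component's world scale, location and forward, right and up vectors into the MPC_Box Material Parameter Collection.
; The values update only when construction runs, as the event graph is empty, and the single shared collection describes one box at a time.
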(fn `UserConstructionScript`
  (bind _cube (`self.Cube`))
  (bind _cube_2 (`self.Cube`))
  (`KismetMaterialLibrary.SetVectorParameterValue` "/Game/Materials/Dissolve/MPC_Box.MPC_Box" "Bounds" (`KismetMathLibrary.Conv_VectorToLinearColor` (`SceneComponent.K2_GetComponentScale` _cube_2)))
  (`KismetMaterialLibrary.SetVectorParameterValue` "/Game/Materials/Dissolve/MPC_Box.MPC_Box" "Location" (`KismetMathLibrary.Conv_VectorToLinearColor` (`SceneComponent.K2_GetComponentLocation` _cube_2)))
  (`KismetMaterialLibrary.SetVectorParameterValue` "/Game/Materials/Dissolve/MPC_Box.MPC_Box" "X" (`KismetMathLibrary.Conv_VectorToLinearColor` (`SceneComponent.GetForwardVector` _cube)))
  (`KismetMaterialLibrary.SetVectorParameterValue` "/Game/Materials/Dissolve/MPC_Box.MPC_Box" "Y" (`KismetMathLibrary.Conv_VectorToLinearColor` (`SceneComponent.GetRightVector` _cube)))
  (`KismetMaterialLibrary.SetVectorParameterValue` "/Game/Materials/Dissolve/MPC_Box.MPC_Box" "Z" (`KismetMathLibrary.Conv_VectorToLinearColor` (`SceneComponent.GetUpVector` _cube))))