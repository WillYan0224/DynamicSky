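; AN_SpawnFootprint is an animation notify that, going by its name, is meant to place footprints, though it currently only performs the ground trace.
; When the weather is not sunny, it picks the left or right foot bone from CurrentLandingFoot.
; It then line traces 100 units along the mesh's down vector against WorldStatic objects, with persistent debug drawing.
; The trace result is unused, so no footprint is spawned.
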(fn `Received_Notify`
  (params (MeshComp :type "SkeletalMeshComponent Object Reference") (Animation :type "AnimSequenceBase Object Reference") (EventReference :type "AnimNotifyEventReference Structure (by ref)"))
  (returns (ReturnValue :type Boolean))
  (locals (CurrentLandingBoneName :type Name :default "None"))
  (bind _returnvalue (`SceneComponent.GetSocketLocation` (`local.MeshComp`) (`local.CurrentLandingBoneName`)))
  (bind _returnvalue_2 (`/Game/Blueprints/AnimNotify/AnimNotifyMacroLibrary.IsSunny`))
  (if (not _returnvalue_2)
    (switch `/Game/Enum/EFootType` (`self.CurrentLandingFoot`)
      (:`NewEnumerator0`
        (set `local.CurrentLandingBoneName` "foot_l"))
      (:`NewEnumerator1`
        (set `local.CurrentLandingBoneName` "foot_r")))
    (`KismetSystemLibrary.LineTraceSingleForObjects` :`Start` _returnvalue :`End` (+ _returnvalue (* (* (`SceneComponent.GetUpVector` (`local.MeshComp`)) -1.0) 100.0)) :`ObjectTypes` (`|MakeArray` "ObjectTypeQuery1" :!type "EObjectTypeQuery Enum") :`DrawDebugType` "Persistent")
    (return false)))